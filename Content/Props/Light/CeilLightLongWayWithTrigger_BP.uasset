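; A ceiling light prop that can switch itself off when the player walks into its trigger box.
; Box overlaps from testPlayer1_BP, gated by the Trigger flag, start a configurable delay followed by a DoOnce, so the shutoff fires a single time.
; The shutoff plays a 2D light-off sound, zeroes the point light's intensity and swaps a mesh material slot to clean glass.
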(event `self.Box.OnComponentBeginOverlap`
  (params (OverlappedComponent :type "PrimitiveComponent Object Reference") (OtherActor :type "Actor Object Reference") (OtherComp :type "PrimitiveComponent Object Reference") (OtherBodyIndex :type Integer) (bFromSweep :type Boolean) (SweepResult :type "HitResult Structure (by ref)"))
  (cast `/Game/Temp/TempPlayer/testPlayer1_BP` OtherActor)
  (if (`self.trigger`)
    (`KismetSystemLibrary.Delay` (`self.delayTime`))
    (`/Engine/EditorBlueprintResources/StandardMacros.DoOnce` false
      (:`Completed`
        (`GameplayStatics.PlaySound2D` "/Game/Audio/Enviroment/Level/lightOff.lightOff" 1.0 1.0 0.0 null null)
        (`LightComponent.SetIntensity` (`self.PointLight`) 0.0)
        (`PrimitiveComponent.SetMaterial` (`self.StaticMesh`) 1 "/Game/Props/Light/Mats/Materials/Free/Glass/M_Glass_Clean.M_Glass_Clean")))))

(fn `UserConstructionScript`
  (`parent.UserConstructionScript`))