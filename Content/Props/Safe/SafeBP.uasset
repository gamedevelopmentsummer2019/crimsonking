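; Interactable safe prop that asks for a passcode before giving access to the item inside.
; Interacting while locked and standing still opens the GameInstance's password widget with this safe's Passcode; the item's collision stays off until unlock.
; Tick polls the widget's IsCorrected flag, then runs a one-shot timed sequence restoring the HUD, playing unlock and door-open level sequences, enabling item pickup and disabling the Box collision.
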(event `self.ReceiveBeginPlay`
  (bind _item (`self.Item`))
  (bind _astest_player_1_bp (cast `/Game/Temp/TempPlayer/testPlayer1_BP` (`GameplayStatics.GetPlayerPawn` 0)))
  (set `self.PlayerPawn` _astest_player_1_bp)
  (bind _ascrimson_game_instance (cast `/Game/MapAndWidget/CrimsonGameInstance` (`GameplayStatics.GetGameInstance`)))
  (set `self.GameInstance` _ascrimson_game_instance)
  (`/Engine/EditorBlueprintResources/StandardMacros.IsValid` _item
    (:`Is Valid`
      (`PrimitiveComponent.SetCollisionEnabled` (`/Game/Gideon/Blueprints/Inventory/Items/itemBase.Sphere` _item) "NoCollision"))))

(event `/Game/Gideon/Blueprints/Interaction/BPI_Interactable.TriggerInteractEvent`
  (if (`self.isLocked`)
    (if (== (`self.GetVelocity` (`GameplayStatics.GetPlayerCharacter` 0)) (0.0 0.0 0.0) :`ErrorTolerance` 0.0)
      (`/Game/MapAndWidget/CrimsonGameInstance.showPasswordInput` (`self.GameInstance`))
      (set `/Game/MapAndWidget/Widget/PasswordInputHUD.correctPassword` (`self.Passcode`) (`/Game/MapAndWidget/CrimsonGameInstance.passwordInput` (`self.GameInstance`))))))

(event `self.ReceiveTick`
  (params (DeltaSeconds :type "Float (single-precision)"))
  (bind _item (`self.Item`))
  (bind _passwordinput (`/Game/MapAndWidget/CrimsonGameInstance.passwordInput` (`self.GameInstance`)))
  (`/Engine/EditorBlueprintResources/StandardMacros.IsValid` _passwordinput
    (:`Is Valid`
      (if (`/Game/MapAndWidget/Widget/PasswordInputHUD.isCorrected` _passwordinput)
        (`/Engine/EditorBlueprintResources/StandardMacros.DoOnce` false
          (:`Completed`
            (`KismetSystemLibrary.Delay` 0.5)
            (`WidgetLayoutLibrary.RemoveAllWidgets`)
            (`/Game/MapAndWidget/CrimsonGameInstance.showPlayerHUD` (`self.GameInstance`))
            (`MovieSceneSequencePlayer.Play` (`ActorSequenceComponent.SequencePlayer` (`self.UnlockSafeAS`)))
            (`KismetSystemLibrary.Delay` 0.8)
            (`/Engine/EditorBlueprintResources/StandardMacros.IsValid` _item
              (:`Is Valid`
                (`PrimitiveComponent.SetCollisionEnabled` (`/Game/Gideon/Blueprints/Inventory/Items/itemBase.Sphere` _item) "QueryAndPhysics"))
              (:`Is Not Valid`
                _))
            (`MovieSceneSequencePlayer.Play` (`ActorSequenceComponent.SequencePlayer` (`self.DoorOpenAS`)))
            (`KismetSystemLibrary.Delay` 1.0)
            (`PrimitiveComponent.SetCollisionEnabled` (`self.Box`) "NoCollision")
            (set `self.isLocked` false)
            (set `/Game/MapAndWidget/Widget/PasswordInputHUD.isCorrected` false (`/Game/MapAndWidget/CrimsonGameInstance.passwordInput` (`self.GameInstance`)))))))))

(fn `UserConstructionScript`)