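; Interactable keyboard prop that opens the exit door and advances the objective.
; Its one-shot interact event disables player input, prints a debug greeting and plays a typing sound, then after a delay calls ExitDoorOpen, restores input and calls NextObjective on the CrimsonGameInstance.
; Tick checks player distance and toggles custom depth on the keyboard and its child components while the player is nearby, likely for highlighting.
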(event `/Game/Gideon/Blueprints/Interaction/BPI_Interactable.TriggerInteractEvent`
  (bind _returnvalue (`GameplayStatics.GetPlayerController` 0))
  (bind _returnvalue_2 (`GameplayStatics.GetPlayerCharacter` 0))
  (`/Engine/EditorBlueprintResources/StandardMacros.DoOnce` false
    (:`Completed`
      (`self.DisableInput` _returnvalue_2 _returnvalue)
      (`KismetSystemLibrary.PrintString` "Hello")
      (`GameplayStatics.PlaySound2D` "/Game/Audio/Enviroment/Level/typing.typing" 1.0 1.0 0.0 null null)
      (`KismetSystemLibrary.Delay` 2.7)
      (`/Engine/EditorBlueprintResources/StandardMacros.DoOnce` false
        (:`Completed`
          (`self.exitDoorOpen`)
          (`self.EnableInput` _returnvalue_2 _returnvalue)
          (bind _ascrimson_game_instance (cast `/Game/MapAndWidget/CrimsonGameInstance` (`GameplayStatics.GetGameInstance`)))
          (`/Game/MapAndWidget/CrimsonGameInstance.nextObjective` _ascrimson_game_instance))))))

(event `self.ReceiveTick`
  (params (DeltaSeconds :type "Float (single-precision)"))
  (bind _inrange (`self.inRange`))
  (set `self.inRange` (< (`KismetMathLibrary.VSize` (- (`self.K2_GetActorLocation`) (`self.K2_GetActorLocation` (`GameplayStatics.GetPlayerCharacter` 0)))) 500.0))
  (for _array_element (`SceneComponent.GetChildrenComponents` (`self.keyboard`) false)
    (bind _asprimitive_component (cast `PrimitiveComponent` _array_element))
    (`PrimitiveComponent.SetRenderCustomDepth` _asprimitive_component _inrange)
    (`PrimitiveComponent.SetRenderCustomDepth` (`self.keyboard`) _inrange)))

(fn `UserConstructionScript`)