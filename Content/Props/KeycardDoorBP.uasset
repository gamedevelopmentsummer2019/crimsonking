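; Keycard door prop that, while locked, opens when the player interacts and can use the required item from their inventory.
; On interact, it asks the player's InventoryComponent to use the item, then once only plays access and unlock sounds, turns its light green and runs an ActorSequence.
; After a short delay it disables collision on an invisible wall.
; Without the item, it briefly shows a locked message on the tutorial HUD.
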(event `self.ReceiveBeginPlay`
  (bind _astest_player_1_bp (cast `/Game/Temp/TempPlayer/testPlayer1_BP` (`GameplayStatics.GetPlayerPawn` 0)))
  (set `self.PlayerPawn` _astest_player_1_bp))

(event `/Game/Gideon/Blueprints/Interaction/BPI_Interactable.TriggerInteractEvent`
  (if (`self.isLocked`)
    (bind _success (`/Game/Gideon/Blueprints/Inventory/Inventory_Component.UseItem` (`/Game/Temp/TempPlayer/testPlayer1_BP.Inventory_Component` (`self.PlayerPawn`)) (`self.ItemNeeded`)))
    (if _success
      (`/Engine/EditorBlueprintResources/StandardMacros.DoOnce` false
        (:`Completed`
          (`GameplayStatics.PlaySoundAtLocation` "/Game/Audio/Enviroment/keycard_access.keycard_access" (`self.K2_GetActorLocation` self) (struct) 3.0 1.0 0.5 null null null)
          (`KismetSystemLibrary.Delay` 1.0)
          (`LightComponent.SetLightColor` (`self.PointLight`) (struct :`R` 0.089607 :`G` 1.0 :`A` 1.0) true)
          (`GameplayStatics.PlaySoundAtLocation` "/Game/Audio/Enviroment/door_unlock.door_unlock" (0.0 0.0 0.0) (struct) 1.0 1.0 0.5 null null null)
          (`MovieSceneSequencePlayer.Play` (`ActorSequenceComponent.SequencePlayer` (`self.ActorSequence`)))
          (`KismetSystemLibrary.Delay` 1.0)
          (`PrimitiveComponent.SetCollisionEnabled` (`self.InviWall`) "NoCollision")))
      (else
        (bind _ashud_tutorial (cast `/Game/Gideon/Blueprints/Tutorial/HUD_Tutorial` (`/Game/Temp/TempPlayer/testPlayer1_BP.TutorialWidget` (`self.PlayerPawn`))))
        (`/Game/Gideon/Blueprints/Tutorial/HUD_Tutorial.SetText` _ashud_tutorial (`self.TextNotifyPlayeWhenItsLock`))
        (`KismetSystemLibrary.Delay` 1.0)
        (`/Game/Gideon/Blueprints/Tutorial/HUD_Tutorial.SetText` _ashud_tutorial "")))))

(fn `UserConstructionScript`)