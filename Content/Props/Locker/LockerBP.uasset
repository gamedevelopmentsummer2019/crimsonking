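; Locker prop that lets the player hide from AI, toggling in or out on each interact event.
; Interacting disables input, activates the LockerOpen sequence component and plays it forward then reversed before restoring input.
; The component's activation event drives the toggle, blending the camera between pawn and locker.
; Entering hides, freezes and teleports the pawn to PlayerLocation; exiting restores visibility and movement after a delay.
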(event `self.ReceiveBeginPlay`
  (bind _astest_player_1_bp (cast `/Game/Temp/TempPlayer/testPlayer1_BP` (`GameplayStatics.GetPlayerPawn` 0)))
  (set `self.PlayerPawn` _astest_player_1_bp))

(event `/Game/Gideon/Blueprints/Interaction/BPI_Interactable.TriggerInteractEvent`
  (bind _lockeropen (`self.LockerOpen`))
  (bind _sequenceplayer (`ActorSequenceComponent.SequencePlayer` _lockeropen))
  ;[1 1 1] Play actionsequence when player interact with the locker
  (`self.DisableInput` (`self.PlayerPawn`) (`GameplayStatics.GetPlayerController` 0))
  (`/Engine/EditorBlueprintResources/StandardMacros.IsValid` _sequenceplayer
    (:`Is Valid`
      (`ActorComponent.Activate` _lockeropen false)
      (`MovieSceneSequencePlayer.Play` _sequenceplayer)
      (`KismetSystemLibrary.Delay` 1.0)
      (`MovieSceneSequencePlayer.PlayReverse` _sequenceplayer)
      (`KismetSystemLibrary.Delay` 1.0)
      (`ActorComponent.Deactivate` (`self.LockerOpen`))
      (`self.EnableInput` (`self.PlayerPawn`) (`GameplayStatics.GetPlayerController` 0)))))

(event `self.LockerOpen.OnComponentActivated`
  (params (Component :type "ActorComponent Object Reference") (bReset :type Boolean))
  (bind _returnvalue (`GameplayStatics.GetPlayerController` 0))
  (bind _playerpawn (`self.PlayerPawn`))
  (bind _playerlocation (`self.PlayerLocation`))
  ;[1 1 1] Move camera when action sequence activated
  (if (`self.isPlayerIntheLocker`)
    (set `self.isPlayerIntheLocker` false)
    (`PlayerController.SetViewTargetWithBlend` _returnvalue (`self.PlayerPawn`) 1.0 "VTBlend_Linear" 0.0 false)
    (`KismetSystemLibrary.Delay` 2.0)
    (`self.SetActorHiddenInGame` (`self.PlayerPawn`) false)
    (set `/Game/Temp/TempPlayer/testPlayer1_BP.canMove` true (`self.PlayerPawn`))
    (`self.SetPlayerVisibleFromAI`)
    (else
      (set `self.isPlayerIntheLocker` true)
      (`PlayerController.SetViewTargetWithBlend` _returnvalue self 1.0 "VTBlend_Linear" 0.0 false)
      (`self.SetActorHiddenInGame` (`self.PlayerPawn`) true)
      (`self.HidePlayerFromAI`)
      (set `/Game/Temp/TempPlayer/testPlayer1_BP.canMove` false _playerpawn)
      (`Controller.SetControlRotation` (`GameplayStatics.GetPlayerController` 0) (`SceneComponent.K2_GetComponentRotation` _playerlocation))
      (`self.K2_SetActorLocation` _playerpawn (`SceneComponent.K2_GetComponentLocation` _playerlocation) false true))))

(fn `HidePlayerFromAI`
  (`/Game/Temp/TempPlayer/testPlayer1_BP.HideFromAI` (`self.PlayerPawn`)))

(fn `SetPlayerVisibleFromAI`
  (`/Game/Temp/TempPlayer/testPlayer1_BP.VisibleFromAI` (`self.PlayerPawn`)))

(fn `UserConstructionScript`)