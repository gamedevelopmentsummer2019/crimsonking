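; JanitorGuide_BP is a guide trigger that shows a help tip on the player's tutorial HUD.
; ChildEvent writes HelpTip into the HUD_Tutorial widget held by testPlayer1_BP and sets a Drawn flag to prevent repeats.
; While Drawn, Tick polls the player's overlap with the actor and clears the text and flag once overlap ends.
; BeginPlay disables collision on the Cube, and several events defer to the parent class.
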(event `self.ReceiveBeginPlay`
  (`parent.ReceiveBeginPlay`)
  (`PrimitiveComponent.SetCollisionEnabled` (`self.Cube`) "NoCollision"))

(event `self.ReceiveTick`
  (params (DeltaSeconds :type "Float (single-precision)"))
  (bind _returnvalue (`GameplayStatics.GetPlayerCharacter` 0))
  (`parent.ReceiveTick` DeltaSeconds)
  (if (`self.Drawn`)
    (if (not (`self.IsOverlappingActor` _returnvalue self))
      (set `self.Drawn` false)
      (bind _astest_player_1_bp (cast `/Game/Temp/TempPlayer/testPlayer1_BP` _returnvalue))
      (bind _ashud_tutorial (cast `/Game/Gideon/Blueprints/Tutorial/HUD_Tutorial` (`/Game/Temp/TempPlayer/testPlayer1_BP.TutorialWidget` _astest_player_1_bp)))
      (`/Game/Gideon/Blueprints/Tutorial/HUD_Tutorial.SetText` _ashud_tutorial ""))))

(event `/Game/Gideon/Blueprints/TriggerEvents/TriggerEvent.TriggerEvent`
  (`parent.TriggerEvent`))

(event `/Game/Gideon/Blueprints/TriggerEvents/TriggerEvent.ChildEvent`
  (if (not (`self.Drawn`))
    (bind _astest_player_1_bp (cast `/Game/Temp/TempPlayer/testPlayer1_BP` (`GameplayStatics.GetPlayerCharacter` 0)))
    (bind _ashud_tutorial (cast `/Game/Gideon/Blueprints/Tutorial/HUD_Tutorial` (`/Game/Temp/TempPlayer/testPlayer1_BP.TutorialWidget` _astest_player_1_bp)))
    (`/Game/Gideon/Blueprints/Tutorial/HUD_Tutorial.SetText` _ashud_tutorial (`self.HelpTip`))
    (set `self.Drawn` true)))

(fn `UserConstructionScript`
  (`parent.UserConstructionScript`))