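; Horror sound trigger Blueprint that plays the HorrorViolin cue as a 2D sound.
; It extends a parent trigger, disabling the Box's collision on BeginPlay before running the parent's logic.
; Its ChildEvent prints a "Hello" debug string and plays the sound, with no call to that event in this Blueprint.
; The overlap and Tick events are disabled stubs.
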(event `self.ReceiveBeginPlay`
  (`PrimitiveComponent.SetCollisionEnabled` (`self.Box`) "NoCollision")
  (`parent.ReceiveBeginPlay`))

(event `/Game/Gideon/Blueprints/TriggerEvents/TriggerEvent.ChildEvent`
  (`KismetSystemLibrary.PrintString` "Hello")
  (`GameplayStatics.PlaySound2D` "/Game/Audio/Enviroment/Level/horrorViolin.horrorViolin" 1.0 1.0 0.0 null null))

(fn `UserConstructionScript`
  (`parent.UserConstructionScript`))