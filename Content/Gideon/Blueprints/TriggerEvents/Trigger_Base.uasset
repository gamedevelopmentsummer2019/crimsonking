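; Base trigger actor that fires a child-defined event when the player character overlaps it.
; Tick polls the overlap with player 0 instead of using overlap events, and a Triggered flag limits TriggerEvent to one ChildEvent call.
; With Repeat enabled, the flag clears after Delaytime once Tick finds the player outside, re-arming the trigger.
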(event `self.ReceiveTick`
  (params (DeltaSeconds :type "Float (single-precision)"))
  (`|ExecutionSequence`
    (:`then_0`
      (if (`self.IsOverlappingActor` (`GameplayStatics.GetPlayerCharacter` 0))
        (`self.TriggerEvent`)
        (elif (`self.Repeat`)
          (if (`self.Triggered`)
            (`KismetSystemLibrary.Delay` (`self.Delaytime`))
            (set `self.Triggered` false)))))))

(event `self.TriggerEvent`
  (if (not (`self.Triggered`))
    (set `self.Triggered` true)
    (`self.ChildEvent`)))

(fn `UserConstructionScript`)