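; SchoolDoor is a door actor meant to trigger a Matinee animation from door handles.
; On BeginPlay it finds every DoorHandle in the level and, through BPI_Interactable, binds its DoorTrigger event to each one.
; DoorTrigger calls DoorTriggerAnim, which searches for actors tagged with MatineeName.
; That loop body is empty: the logic to play the first MatineeActor found is disconnected, so no animation plays.
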(event `DoorTriggerAnim`
  ;[1 1 1] Dorr Animation Event
  (bind _outactors (`GameplayStatics.GetAllActorsWithTag` (`KismetStringLibrary.Conv_StringToName` (`self.MatineeName`))))
  (for _array_element _outactors
    _))

(event `self.ReceiveBeginPlay`
  (bind _outactors (`GameplayStatics.GetAllActorsOfClass` "/Game/Gideon/Blueprints/Interaction/DoorHandle.DoorHandle_C"))
  (for _array_element _outactors
    (if (`KismetSystemLibrary.DoesImplementInterface` _array_element "/Game/Gideon/Blueprints/Interaction/BPI_Interactable.BPI_Interactable_C")
      (add `/Game/Gideon/Blueprints/Interaction/DoorHandle.DoorTrigger` _array_element (delegate `DoorTrigger`)))))

(event `DoorTrigger`
  (`self.DoorTriggerAnim`))

(fn `UserConstructionScript`)