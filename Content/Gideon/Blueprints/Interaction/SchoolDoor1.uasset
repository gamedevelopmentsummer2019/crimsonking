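; SchoolDoor1 is a school door that plays a Matinee animation when triggered by a door handle.
; On BeginPlay it finds every DoorHandle1 in the level and, through BPI_Interactable, binds its DoorTrigger event to each one.
; When triggered, it looks up actors tagged with MatineeName and plays the first MatineeActor found, so the animation is linked by tag rather than direct reference.
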(event `DoorTriggerAnim`
  ;[1 1 1] Dorr Animation Event
  (bind _outactors (`GameplayStatics.GetAllActorsWithTag` (`KismetStringLibrary.Conv_StringToName` (`self.MatineeName`))))
  (for _array_element _outactors
    (if (== (`GameplayStatics.GetObjectClass` _array_element) "/Script/Engine.MatineeActor")
      (bind _asmatinee_actor (cast `MatineeActor` _array_element))
      (`MatineeActor.Play` _asmatinee_actor)
      (break))))

(event `self.ReceiveBeginPlay`
  (bind _outactors (`GameplayStatics.GetAllActorsOfClass` "/Game/Gideon/Blueprints/Interaction/DoorHandle1.DoorHandle1_C"))
  (for _array_element _outactors :!label _label
    (if (`KismetSystemLibrary.DoesImplementInterface` _array_element "/Game/Gideon/Blueprints/Interaction/BPI_Interactable.BPI_Interactable_C")
      (add `/Game/Gideon/Blueprints/Interaction/DoorHandle1.DoorTrigger1` _array_element (delegate `DoorTrigger`)))))

(event `DoorTrigger`
  (`self.DoorTriggerAnim`)
  (goto _label :!via `Break`))

(fn `UserConstructionScript`)