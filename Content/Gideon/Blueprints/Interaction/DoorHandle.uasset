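; DoorHandle is an interactable door handle that requires an item from the player's inventory to fire its door trigger.
; TriggerInteractEvent casts player character 0 to testPlayer1_BP, asks its InventoryComponent to use ItemNeeded, and calls DoorTrigger only if that succeeds.
; A failed cast prints a debug string, and an older player_BP cast remains as unreachable leftover.
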(event `/Game/Gideon/Blueprints/Interaction/BPI_Interactable.TriggerInteractEvent`
  (bind _astest_player_1_bp (cast `/Game/Temp/TempPlayer/testPlayer1_BP` (`GameplayStatics.GetPlayerCharacter` 0))
    (:`then`
      (bind _success (`/Game/Gideon/Blueprints/Inventory/Inventory_Component.UseItem` (`/Game/Temp/TempPlayer/testPlayer1_BP.Inventory_Component` _astest_player_1_bp) (`self.ItemNeeded`)))
      (if _success
        (`self.DoorTrigger`)))
    (:`CastFailed`
      (`KismetSystemLibrary.PrintString` "Failed sdadsadsada" true true (struct :`R` 0.894014 :`G` 0.237873 :`B` 1.0 :`A` 1.0)))))

(fn `UserConstructionScript`)