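; Inventory component that holds a fixed number of item slots and toggles a centered inventory window on the player HUD, switching input mode.
; PrepareInventory sizes the slot array and refreshes item data from class defaults on BeginPlay and window open.
; AddToInventory fills partial stacks of stackable items, recursing on overflow, or writes to an empty slot via CreateStack.
; Adding always reports success, with no full-inventory check.
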(event `self.ReceiveBeginPlay`
  (`self.PrepareInventory`))

(fn `AddToInventory`
  (params (ItemToAdd :type "/Game/Gideon/Blueprints/Inventory/SlotStructure Structure"))
  (returns (Success :type Boolean))
  (if (`.IsStackable_17_8CA02B5B45D9D7539BB33D8EEBDE6263` (break `/Game/Gideon/Blueprints/Inventory/ItemStructure` (break `/Game/Gideon/Blueprints/Inventory/SlotStructure` ItemToAdd)))
    (bind _stackindex (`self.HasPartialStack` (`local.ItemToAdd`))
      (:`True`
        (bind _added (`self.AddToStack` (`local.ItemToAdd`) _stackindex))
        (set `self.AddedSuccess` _added))
      (:`false`
        (`self.CreateStack` (`local.ItemToAdd`) :!label _label)
        (set `self.AddedSuccess` true)))
    (else
      (goto _label)))
  (return (`self.AddedSuccess`)))

(fn `AddToStack`
  (params (SlotStructure :type "/Game/Gideon/Blueprints/Inventory/SlotStructure Structure") (SlotIndex :type Integer))
  (returns (Added :type Boolean))
  (locals (CurrentQuantity :type Integer))
  (bind (_itemstructure _quantity) (break `/Game/Gideon/Blueprints/Inventory/SlotStructure` SlotStructure))
  (bind _slotindex (`local.SlotIndex`))
  (bind _inventory (`self.Inventory`))
  (bind _slotstructure_itemstructure (break `/Game/Gideon/Blueprints/Inventory/SlotStructure` (`local.SlotStructure`)))
  (bind (_slotstructure_itemstructure_2 _slotstructure_quantity) (break `/Game/Gideon/Blueprints/Inventory/SlotStructure` (`local.SlotStructure`)))
  (bind (_itemname _isconsumable _isstackable _maxstacksize) (break `/Game/Gideon/Blueprints/Inventory/ItemStructure` _slotstructure_itemstructure))
  (bind _output (`|GetArrayItem` (`self.Inventory`) SlotIndex))
  (bind (_output_itemstructure _output_quantity) (break `/Game/Gideon/Blueprints/Inventory/SlotStructure` (`|GetArrayItem` _inventory _slotindex)))
  (bind _output_get (set `local.CurrentQuantity` (`.Quantity_5_58483AD34B71665D68A9BCB57A2B4206` (break `/Game/Gideon/Blueprints/Inventory/SlotStructure` _output))))
  (if (> (+ _output_get _quantity) (`.MaxStackSize_21_733E2E0A47A87D64F5BC8A99629E3B6F` (break `/Game/Gideon/Blueprints/Inventory/ItemStructure` (break `/Game/Gideon/Blueprints/Inventory/SlotStructure` _output))))
    (`KismetArrayLibrary.Array_Set` (`self.Inventory`) (`local.SlotIndex`) (make `/Game/Gideon/Blueprints/Inventory/SlotStructure` _slotstructure_itemstructure _maxstacksize))
    (`self.AddToInventory` (make `/Game/Gideon/Blueprints/Inventory/SlotStructure` _slotstructure_itemstructure_2 (- _slotstructure_quantity (- (`local.CurrentQuantity`) _maxstacksize))))
    (else
      (`KismetArrayLibrary.Array_Set` _inventory _slotindex (make `/Game/Gideon/Blueprints/Inventory/SlotStructure` _output_itemstructure (+ _output_quantity _quantity)))))
  (return true))

(fn `CreateStack`
  (params (ItemToAdd :type "/Game/Gideon/Blueprints/Inventory/SlotStructure Structure"))
  (bind _inventory (`self.Inventory`))
  (`KismetArrayLibrary.Array_Set` _inventory (`KismetArrayLibrary.Array_Find` _inventory (make `/Game/Gideon/Blueprints/Inventory/SlotStructure` (struct :`itemName` "NSLOCTEXT(\"[52B239F84B741669C3B729B15E8E1D89]\", \"8435C0614AEDA4AAB06A7CABFF8FE211\", \"None\")" :`itemDescription` "NSLOCTEXT(\"[52B239F84B741669C3B729B15E8E1D89]\", \"B73D9A834928138CB9CAC0B9E22C9DA1\", \"None\")" :`MaxStackSize` 4))) ItemToAdd))

(fn `PrepareInventory`
  (`KismetArrayLibrary.Array_Resize` (`self.Inventory`) (`self.NumberofSlots`))
  (for (_array_element _array_index) (`self.Inventory`)
    (bind (_itemname _isconsumable _isstackable _maxstacksize _itemthumbnail _itemdescription _itemclass) (break `/Game/Gideon/Blueprints/Inventory/ItemStructure` (break `/Game/Gideon/Blueprints/Inventory/SlotStructure` _array_element)))
    (if (!= _itemclass null)
      (`KismetArrayLibrary.Array_Set` (`self.Inventory`) _array_index (make `/Game/Gideon/Blueprints/Inventory/SlotStructure` (defaults `/Game/Gideon/Blueprints/Inventory/Inventory_Component` _itemclass) (`.Quantity_5_58483AD34B71665D68A9BCB57A2B4206` (break `/Game/Gideon/Blueprints/Inventory/SlotStructure` _array_element)))))))

(fn `ToggleInventory`
  (`self.InventoryWindow`
    (:`then`
      (`Widget.RemoveFromParent` (`self.InventoryWindow`))
      (set `self.InventoryWindow` null)
      (`WidgetBlueprintLibrary.SetInputMode_GameOnly` (`GameplayStatics.GetPlayerController` 0)))
    (:`else`
      (`self.PrepareInventory`)
      (bind _returnvalue (`|CreateWidget` "/Game/Gideon/Blueprints/Inventory/InventoryUI/Inventory_Window.Inventory_Window_C" null self))
      (set `self.InventoryWindow` _returnvalue)
      (bind _asplayer_controller (cast `/Game/Player/gameModeAndController/playerController` (`GameplayStatics.GetPlayerController` 0)))
      (bind _returnvalue_2 (`CanvasPanel.AddChildToCanvas` (`/Game/Gideon/Blueprints/Inventory/InventoryUI/HUD.Hud_Canvas` (`/Game/Player/gameModeAndController/playerController.HudWidget` _asplayer_controller)) (`self.InventoryWindow`)))
      (`CanvasPanelSlot.SetAutoSize` _returnvalue_2 true)
      (`CanvasPanelSlot.SetAlignment` _returnvalue_2 (0.5 0.5))
      (`CanvasPanelSlot.SetAnchors` _returnvalue_2 (make `Anchors` (0.5 0.5) (0.5 0.5)))
      (`CanvasPanelSlot.SetPosition` _returnvalue_2 (`self.Position`))
      (`WidgetBlueprintLibrary.SetInputMode_UIOnlyEx` (`GameplayStatics.GetPlayerController` 0) (`self.InventoryWindow`) "LockAlways"))))